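; BP_DummyEnemy is a dummy enemy that reports the damage it receives.
; Its AnyDamage event prints the damage amount, damage type, instigator and damage causer as separate log lines.
; It applies no health or reaction logic; a BP_DamageTypeFiire class check and a damage-doubling multiply are left unconnected, and the construction script is empty.
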(event `self.ReceiveAnyDamage`
  (params (Damage :type "Float (single-precision)") (DamageType :type "DamageType Object Reference") (InstigatedBy :type "Controller Object Reference") (DamageCauser :type "Actor Object Reference"))
  (`KismetSystemLibrary.LogString` (`KismetStringLibrary.BuildString_Double` "" "Damage : " Damage))
  (`KismetSystemLibrary.LogString` (`KismetStringLibrary.Concat_StrStr` "DamageType : " (`KismetSystemLibrary.GetDisplayName` DamageType)))
  (`KismetSystemLibrary.LogString` (`KismetStringLibrary.Concat_StrStr` "Instigate : " (`KismetSystemLibrary.GetDisplayName` InstigatedBy)))
  (`KismetSystemLibrary.LogString` (`KismetStringLibrary.Concat_StrStr` "Damage Causer : " (`KismetSystemLibrary.GetDisplayName` DamageCauser))))

(fn `UserConstructionScript`)